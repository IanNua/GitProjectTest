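; BP_Sam_Character is a character Blueprint that nudges itself to a random nearby position when play begins.
; BeginPlay runs a Sequence that starts a retriggerable delay with nothing wired after it, then immediately calls Funny.
; Funny teleports the actor without sweep by a random positive X and Y offset of up to 100 units each, leaving Z unchanged.
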(event EventBeginPlay
  (Utilities|FlowControl|Sequence
    (:then_0
      (Utilities|FlowControl|RetriggerableDelay 1.0))
    (:then_1
      (CallFunction|Funny))))

(fn ConstructionScript)

(fn Funny
  (Transformation|SetActorLocation (+ (Transformation|GetActorLocation) (Math|Vector|MakeVector (* (Math|Random|RandomFloat) 1e+02) (* (Math|Random|RandomFloat) 1e+02) 0.0)) false true))