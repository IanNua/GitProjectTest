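; BP_Character_Nye is a short-lived actor that spawns another actor shortly after play begins, then destroys itself.
; BeginPlay starts a one-shot timer for the Shoot event and uses a longer delay before destruction.
; Shoot spawns the given class at SpawnCube's location, then offsets itself by the spawned actor's world X and Y plus a small constant.
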(event Custom|Shoot
  (bind _returnvalue (Game|SpawnActorfromClass (Variables|Default|GetClass) (Math|Transform|MakeTransform (Transformation|GetWorldLocation (Variables|Default|GetSpawn%20Cube)) "0, 0, 0" "1.000000,1.000000,1.000000") "Undefined" "MultiplyWithRoot" 0 0))
  (Transformation|AddActorWorldOffset (Math|Vector|MakeVector (+ (.x (Transformation|GetWorldLocation (Variables|/Script/Engine.Actor|GetRootComponent _returnvalue))) 2.0) (+ (.y (Transformation|GetWorldLocation (Variables|/Script/Engine.Actor|GetRootComponent _returnvalue))) 2.0) 0.0)))

(event EventBeginPlay
  (Utilities|Time|SetTimerbyEvent (delegate Custom|Shoot) 1.0)
  (Utilities|FlowControl|Delay 2.0)
  (Actor|DestroyActor))

(event Collision|EventActorBeginOverlap
  (params (OtherActor :type Actor%20Object%20Reference)))

(fn ConstructionScript)